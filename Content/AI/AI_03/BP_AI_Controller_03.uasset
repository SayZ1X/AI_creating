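; BP_AI_Controller_03 is an AI controller that patrols its controlled pawn through TargetPoint actors tagged "playground_1".
; Every Tick gathers the tagged points, issues AIMoveTo toward the current index and draws a debug sphere there.
; On success the index increments; at the end it wraps to zero and moves again immediately, otherwise movement stops until Tick reissues it.
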(event `self.ReceiveTick`
  (params (DeltaSeconds :type "Float (single-precision)"))
  ;[1 1 1] patrooling
  (bind _outactors (`GameplayStatics.GetAllActorsOfClassWithTag` "/Script/Engine.TargetPoint" "playground_1"))
  (bind _output (`|GetArrayItem` _outactors (`self.Patroling_Points`)))
  (`|AIMoveTo` (`self.K2_GetPawn`) (0.0 0.0 0.0) _output :!label _label
    (:`then`
      (`KismetSystemLibrary.DrawDebugSphere` (`self.K2_GetActorLocation` _output) 30.0 16 (struct :`R` 1.0 :`B` 0.056108 :`A` 1.0)))
    (:`OnSuccess`
      (bind _result (`/Engine/EditorBlueprintResources/StandardMacros.IncrementInt` (`self.Patroling_Points`))
        (:`  `
          (bind _output_get (set `self.Patroling_Points` _result))
          (if (== _output_get (`KismetArrayLibrary.Array_Length` _outactors))
            (set `self.Patroling_Points` 0)
            (goto _label)
            (else
              (`self.StopMovement`))))))))

(event `self.ReceiveBeginPlay`)

(fn `UserConstructionScript`)