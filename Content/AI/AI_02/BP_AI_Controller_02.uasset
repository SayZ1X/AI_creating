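; BP_AI_Controller_02 is an AI controller that sends its pawn to a tagged destination when play begins.
; On BeginPlay it finds the first actor tagged "playground_2" and calls MoveToLocation on its position, pathing through the custom BP_Nav_Query_Filter_1 navigation filter.
; Two unconnected alternatives remain in the graph: a simple move to the same location and a simple move to the player pawn.
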(event `self.ReceiveTick`
  (params (DeltaSeconds :type "Float (single-precision)")))

(event `self.ReceiveBeginPlay`
  ;[1 1 1] Move to actor expendet
  (bind _outactors (`GameplayStatics.GetAllActorsWithTag` "playground_2"))
  (`self.MoveToLocation` (`self.K2_GetActorLocation` (`|GetArrayItem` _outactors)) -1.0 true true false true "/Game/AI/Navigation_Query_Filters/BP_Nav_Query_Filter_1.BP_Nav_Query_Filter_1_C"))

(fn `UserConstructionScript`)