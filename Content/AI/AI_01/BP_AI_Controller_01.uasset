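; AI controller that keeps its pawn moving along a stored Direction and randomly steers it when something is ahead.
; Each Tick runs a debug-drawn Visibility line trace along the pawn's forward vector, ignoring the pawn itself.
; While the trace hits, Direction yaws a small step left or right, with the side re-rolled every frame.
; Direction then feeds AddMovementInput every frame, with or without a hit.
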(event `self.ReceiveTick`
  (params (DeltaSeconds :type "Float (single-precision)"))
  (bind _returnvalue (`self.K2_GetPawn`))
  (bind _returnvalue_2 (`self.K2_GetActorLocation` _returnvalue))
  (bind (_outhit _returnvalue_3) (`KismetSystemLibrary.LineTraceSingle` _returnvalue_2 (+ _returnvalue_2 (* (`self.GetActorForwardVector` _returnvalue) 800)) "TraceTypeQuery1" false (`|MakeArray` (`self.K2_GetPawn`) :!type "Actor Object Reference") "ForOneFrame" true (struct :`R` 1.0 :`A` 1.0) (struct :`R` 0.102331 :`G` 1.0 :`A` 1.0)))
  (if _returnvalue_3
    (set `self.Random_Rotation` (`KismetMathLibrary.SelectFloat` 4.0 -4.0 (`KismetMathLibrary.RandomBool`)))
    (bind _output_get (set `self.Direction` (`KismetMathLibrary.GreaterGreater_VectorRotator` (`self.Direction`) (`KismetMathLibrary.MakeRotator` 0.0 0.0 (`self.Random_Rotation`))))))
  (`Pawn.AddMovementInput` (`self.K2_GetPawn`) _output_get 1.0 false))

(fn `UserConstructionScript`)