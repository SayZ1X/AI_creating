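; AI controller for the AI_08 agent that starts the BT_Main_08 behavior tree on possess.
; AI Perception sight updates write the sensed actor to the "Player" blackboard key and clear it when sight is lost, without checking which actor it is.
; Damage stimuli only print their strength to screen and do not affect the blackboard.
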(event `self.ReceiveBeginPlay`)

(event `self.ReceiveTick`
  (params (DeltaSeconds :type "Float (single-precision)")))

(event `self.ReceivePossess`
  (params (PossessedPawn :type "Pawn Object Reference"))
  (`self.RunBehaviorTree` "/Game/AI/AI_08/BT_Main_08.BT_Main_08"))

(event `self.AIPerception.OnTargetPerceptionUpdated`
  (params (Actor :type "Actor Object Reference") (Stimulus :type "AIStimulus Structure"))
  (bind _returnvalue (`AIPerceptionSystem.GetSenseClassForStimulus` Stimulus))
  (if (== _returnvalue "/Script/AIModule.AISense_Sight")
    (if (`.bSuccessfullySensed` (break `AIStimulus` Stimulus))
      (`BlackboardComponent.SetValueAsObject` (`AIBlueprintHelperLibrary.GetBlackboard` null) (`KismetStringLibrary.Conv_StringToName` "Player") Actor)
      (else
        (`BlackboardComponent.ClearValue` (`AIBlueprintHelperLibrary.GetBlackboard` null) (`KismetStringLibrary.Conv_StringToName` "Player"))))))

(event `self.AIPerception.OnTargetPerceptionInfoUpdated`
  (params (UpdateInfo :type "ActorPerceptionUpdateInfo Structure (by ref)"))
  (bind (_targetid _target _stimulus) (break `ActorPerceptionUpdateInfo` UpdateInfo))
  (bind _returnvalue (`AIPerceptionSystem.GetSenseClassForStimulus` _stimulus))
  (if (== _returnvalue "/Script/AIModule.AISense_Damage")
    (`KismetSystemLibrary.PrintString` (`KismetStringLibrary.Conv_DoubleToString` (`.Strength` (break `AIStimulus` _stimulus))))))

(fn `UserConstructionScript`)