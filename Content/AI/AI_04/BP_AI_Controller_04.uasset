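; AI controller that walks its pawn through a one-pass patrol of level actors tagged "playground_3".
; On BeginPlay it gathers the tagged actors and runs AI MoveTo to the location at the PatrolingPoints index.
; Each success increments the index and repeats until the array ends, with no wraparound or failure handling.
; Unconnected nodes hold simpler SimpleMoveToLocation and SimpleMoveToActor variants that never run.
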(event `self.ReceiveBeginPlay`
  ;[1 1 1] Move to actor expendet
  (bind _outactors (`GameplayStatics.GetAllActorsWithTag` "playground_3"))
  (`|AIMoveTo` null (`self.K2_GetActorLocation` (`|GetArrayItem` _outactors (`self.Patroling_Points`))) null :!label _label
    (:`OnSuccess`
      (bind _result (`/Engine/EditorBlueprintResources/StandardMacros.IncrementInt` (`self.Patroling_Points`))
        (:`  `
          (bind _output_get (set `self.Patroling_Points` _result))
          (if (< _output_get (`KismetArrayLibrary.Array_Length` _outactors))
            (goto _label)))))))

(event `self.ReceiveTick`
  (params (DeltaSeconds :type "Float (single-precision)")))

(fn `UserConstructionScript`)